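; BP_Barman is a bartender character that varies its appearance each time it spawns.
; On BeginPlay it assigns a random mesh from an array to StaticMesh1 and a random material from an array to the first slot of StaticMesh.
; It then plays a single looping animation directly on its Mesh.
; Tick and the construction script are empty.
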(event EventBeginPlay
  (Components|StaticMesh|SetStaticMesh (Variables|Default|GetStaticMesh1) (.OutItem (Utilities|Array|Random (Variables|Default|GetNew%20Mesh))))
  (Rendering|Material|SetMaterial (Variables|Default|GetStaticMesh) 0 (.OutItem (Utilities|Array|Random (Variables|Default|GetMaterial))))
  (Components|Animation|PlayAnimation (Variables|Character|GetMesh) (Variables|Default|GetNew%20Anim%20to%20Play) true))

(event EventTick
  (params (DeltaSeconds :type Float%20%28single-precision%29)))

(fn ConstructionScript)