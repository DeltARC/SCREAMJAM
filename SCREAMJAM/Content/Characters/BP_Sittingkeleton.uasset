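; BP_Sittingkeleton is a character Blueprint, by its name a sitting skeleton, dressed with randomized static meshes.
; On BeginPlay it picks random meshes for two components and assigns a set mesh to a third.
; When the first matches a specific glasses mesh (LunettesBG__3_), it also gets a random material.
; The main mesh then loops a configurable animation, with no Tick or construction logic.
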(event EventBeginPlay
  (Components|StaticMesh|SetStaticMesh (Variables|Default|GetStaticMesh) (.OutItem (Utilities|Array|Random (Variables|Default|GetNew%20Mesh_0))))
  (Components|StaticMesh|SetStaticMesh (Variables|Default|GetStaticMesh1) (.OutItem (Utilities|Array|Random (Variables|Default|GetNew%20Mesh))))
  (if (== (Variables|Default|GetStaticMesh) "/Game/Characters/LunettesBG__3_.LunettesBG__3_")
    (Rendering|Material|SetMaterial (Variables|Default|GetStaticMesh) 0 (.OutItem (Utilities|Array|Random (Variables|Default|GetMaterial)))))
  (Components|StaticMesh|SetStaticMesh (Variables|Default|GetStaticMesh2) (Variables|Default|GetNew%20Mesh_2))
  (Components|Animation|PlayAnimation (Variables|Character|GetMesh) (Variables|Default|GetNew%20Anim%20to%20Play) true))

(event EventTick
  (params (DeltaSeconds :type Float%20%28single-precision%29)))

(fn ConstructionScript)