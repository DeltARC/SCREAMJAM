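; Test actor for a music ordering mechanic that requests one of three tracks and judges the one played.
; A looping five-second timer starts an order when idle, updating a WBP_Order image.
; The displayed texture is randomized independently of the ordered track index, and the widget is never added to the viewport here.
; VerifyMusic compares the played index, briefly shows match or mismatch on image and cylinder, then clears the order.
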(event Custom|Order
  (bind _returnvalue (Math|Random|RandomIntegerinRange 0 2))
  (if (not (Variables|Default|GetIsOrdering))
    (bind _output_get (Variables|Default|SetOrderedMusic _returnvalue))
    (Development|PrintString (Utilities|String|ToString(Integer) _output_get))
    (Variables|Default|SetIsOrdering true)
    (Appearance|SetBrushfromTexture (Variables|/Game/Widgets/WBP_Order.WBP_Order_C|GetImage_59 (Variables|Default|GetOrder%20Ref)) (Utilities|Array|Get(acopy) (Variables|Default|GetTextureOrder) _returnvalue) false)))

(event Custom|VerifyMusic
  (params (PlayedMusic :type Integer))
  (if (Variables|Default|GetIsOrdering)
    (if (== PlayedMusic (Variables|Default|GetOrderedMusic))
      (Rendering|Material|SetMaterial (Variables|Default|GetCylinder) 0 "/Game/Materials/M_Emoji.M_Emoji")
      (Appearance|SetBrushfromTexture (Variables|/Game/Widgets/WBP_Order.WBP_Order_C|GetImage_59 (Variables|Default|GetOrder%20Ref)) "/Game/Materials/T_Emoji.T_Emoji" false)
      (Utilities|FlowControl|Delay 3.0)
      (Appearance|SetBrushfromTexture (Variables|/Game/Widgets/WBP_Order.WBP_Order_C|GetImage_59 (Variables|Default|GetOrder%20Ref)) "/Engine/ArtTools/RenderToTexture/Textures/127grey.127grey" false)
      (Rendering|Material|SetMaterial (Variables|Default|GetCylinder) 0 "/Game/Characters/Material.Material")
      (Variables|Default|SetIsOrdering false)
      (else
        (Rendering|Material|SetMaterial (Variables|Default|GetCylinder) 0 "/Game/Materials/M_TripleT.M_TripleT")
        (Appearance|SetBrushfromTexture (Variables|/Game/Widgets/WBP_Order.WBP_Order_C|GetImage_59 (Variables|Default|GetOrder%20Ref)) "/Game/Materials/T_TripleT.T_TripleT" false)
        (Utilities|FlowControl|Delay 3.0)
        (Appearance|SetBrushfromTexture (Variables|/Game/Widgets/WBP_Order.WBP_Order_C|GetImage_59 (Variables|Default|GetOrder%20Ref)) "/Engine/ArtTools/RenderToTexture/Textures/127grey.127grey" false)
        (Rendering|Material|SetMaterial (Variables|Default|GetCylinder) 0 "/Game/Characters/Material.Material")
        (Variables|Default|SetIsOrdering false)))))

(event EventBeginPlay
  (bind _returnvalue (Math|Random|RandomIntegerinRange 0 2))
  (bind _returnvalue_2 (UserInterface|CreateWidget "/Game/Widgets/WBP_Order.WBP_Order_C"))
  (Variables|Default|SetOrder%20Ref _returnvalue_2)
  (Utilities|Time|SetTimerbyEvent (delegate Custom|Order) 5.0 true)
  (if (not (Variables|Default|GetIsOrdering))
    (bind _output_get (Variables|Default|SetOrderedMusic _returnvalue))
    (Development|PrintString (Utilities|String|ToString(Integer) _output_get))
    (Variables|Default|SetIsOrdering true)
    (Appearance|SetBrushfromTexture (Variables|/Game/Widgets/WBP_Order.WBP_Order_C|GetImage_59 (Variables|Default|GetOrder%20Ref)) (Utilities|Array|Get(acopy) (Variables|Default|GetTextureOrder) _returnvalue) false)))

(fn ConstructionScript)