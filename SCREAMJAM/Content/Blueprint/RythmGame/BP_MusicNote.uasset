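; BP_MusicNote is a moving note actor for the rhythm game, represented by a Cube component.
; On BeginPlay it finds the BP_Screen actor, stores it and starts a Timeline.
; Each update moves the Cube along the screen's Arrow1 forward vector, scaled by Multiplicator.
; The lerp starts from the current location, so each step accumulates, with the Timeline track setting step size rather than absolute position.
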(event EventBeginPlay
  (bind _cube (Variables|Default|GetCube))
  (bind _returnvalue (Transformation|GetWorldLocation _cube))
  (bind _returnvalue_2 (Actor|GetActorOfClass "/Game/Blueprint/RythmGame/BP_Screen.BP_Screen_C"))
  (Variables|Default|SetScreenRef _returnvalue_2)
  (bind _newtrack_0 (Timeline|Timeline PlayFromStart)
    (:Update
      (Transformation|SetWorldLocation _cube (Math|Vector|Lerp(Vector) _returnvalue (+ _returnvalue (* (Math|Vector|GetForwardVector (Variables|/Game/Blueprint/RythmGame/BP_Screen.BP_Screen_C|GetArrow%201 (Variables|Default|GetScreenRef))) (Variables|Default|Getmultiplicator))) _newtrack_0) false false))))

(fn ConstructionScript)