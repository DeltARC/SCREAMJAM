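; BP_Screen is the rhythm game screen that spawns music notes in three lanes and judges their timing window.
; LaunchGame starts a looping one-second timer that spawns one or two BP_MusicNote actors at random lane arrows.
; Overlap zones S1–S3 toggle the first-person character's per-lane "Good" flags.
; Notes leaving a zone are hidden by their overlapping component, and trigger FailedNote on the character if that lane wasn't clicked.
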(event OnComponentBeginOverlap(s1)
  (params (OverlappedComponent :type Primitive%20Component%20Object%20Reference) (OtherActor :type Actor%20Object%20Reference) (OtherComp :type Primitive%20Component%20Object%20Reference) (OtherBodyIndex :type Integer) (bFromSweep :type Boolean) (SweepResult :type Hit%20Result%20Structure%20%28by%20ref%29))
  ;[0.15 0.15 0.15 0.5] Notes valides ou pas
  (Variables|/Game/FirstPerson/Blueprints/BP_FirstPersonCharacter.BP_FirstPersonCharacter_C|SetMusicNote1%20Good (Variables|Default|GetAs%20BP%20First%20Person%20Character) true))

(event OnComponentEndOverlap(s1)
  (params (OverlappedComponent :type Primitive%20Component%20Object%20Reference) (OtherActor :type Actor%20Object%20Reference) (OtherComp :type Primitive%20Component%20Object%20Reference) (OtherBodyIndex :type Integer))
  (bind _as_bp_first_person_character (Variables|Default|GetAs%20BP%20First%20Person%20Character))
  ;[0.15 0.15 0.15 0.5] Notes valides ou pas
  (Variables|/Game/FirstPerson/Blueprints/BP_FirstPersonCharacter.BP_FirstPersonCharacter_C|SetMusicNote1%20Good _as_bp_first_person_character false)
  (Rendering|SetVisibility OtherComp false false)
  (if (not (Variables|/Game/FirstPerson/Blueprints/BP_FirstPersonCharacter.BP_FirstPersonCharacter_C|Getnote%201%20clicked _as_bp_first_person_character))
    (Default|FailedNote _as_bp_first_person_character)))

(event OnComponentEndOverlap(s2)
  (params (OverlappedComponent :type Primitive%20Component%20Object%20Reference) (OtherActor :type Actor%20Object%20Reference) (OtherComp :type Primitive%20Component%20Object%20Reference) (OtherBodyIndex :type Integer))
  (bind _as_bp_first_person_character (Variables|Default|GetAs%20BP%20First%20Person%20Character))
  ;[0.15 0.15 0.15 0.5] Notes valides ou pas
  (Variables|/Game/FirstPerson/Blueprints/BP_FirstPersonCharacter.BP_FirstPersonCharacter_C|SetMusicNote2%20Good _as_bp_first_person_character false)
  (Rendering|SetVisibility OtherComp false false)
  (if (not (Variables|/Game/FirstPerson/Blueprints/BP_FirstPersonCharacter.BP_FirstPersonCharacter_C|Getnote%202%20clicked _as_bp_first_person_character))
    (Default|FailedNote _as_bp_first_person_character)))

(event OnComponentEndOverlap(s3)
  (params (OverlappedComponent :type Primitive%20Component%20Object%20Reference) (OtherActor :type Actor%20Object%20Reference) (OtherComp :type Primitive%20Component%20Object%20Reference) (OtherBodyIndex :type Integer))
  (bind _as_bp_first_person_character (Variables|Default|GetAs%20BP%20First%20Person%20Character))
  ;[0.15 0.15 0.15 0.5] Notes valides ou pas
  (Variables|/Game/FirstPerson/Blueprints/BP_FirstPersonCharacter.BP_FirstPersonCharacter_C|SetMusicNote3%20Good _as_bp_first_person_character false)
  (Rendering|SetVisibility OtherComp false false)
  (if (not (Variables|/Game/FirstPerson/Blueprints/BP_FirstPersonCharacter.BP_FirstPersonCharacter_C|Getnote%203%20clicked _as_bp_first_person_character))
    (Default|FailedNote _as_bp_first_person_character)))

(event OnComponentBeginOverlap(s2)
  (params (OverlappedComponent :type Primitive%20Component%20Object%20Reference) (OtherActor :type Actor%20Object%20Reference) (OtherComp :type Primitive%20Component%20Object%20Reference) (OtherBodyIndex :type Integer) (bFromSweep :type Boolean) (SweepResult :type Hit%20Result%20Structure%20%28by%20ref%29))
  ;[0.15 0.15 0.15 0.5] Notes valides ou pas
  (Variables|/Game/FirstPerson/Blueprints/BP_FirstPersonCharacter.BP_FirstPersonCharacter_C|SetMusicNote2%20Good (Variables|Default|GetAs%20BP%20First%20Person%20Character) true))

(event OnComponentBeginOverlap(s3)
  (params (OverlappedComponent :type Primitive%20Component%20Object%20Reference) (OtherActor :type Actor%20Object%20Reference) (OtherComp :type Primitive%20Component%20Object%20Reference) (OtherBodyIndex :type Integer) (bFromSweep :type Boolean) (SweepResult :type Hit%20Result%20Structure%20%28by%20ref%29))
  ;[0.15 0.15 0.15 0.5] Notes valides ou pas
  (Variables|/Game/FirstPerson/Blueprints/BP_FirstPersonCharacter.BP_FirstPersonCharacter_C|SetMusicNote3%20Good (Variables|Default|GetAs%20BP%20First%20Person%20Character) true))

(event Custom|music%20note%20spawn
  (bind _returnvalue (Math|Random|RandomIntegerinRange 1 3))
  (bind _returnvalue_2 (Math|Random|RandomIntegerinRange 1 3))
  ;[0.15 0.15 0.15 0.5] spawn des notes
  (if (== (Math|Random|RandomIntegerinRange 1 2) 1)
    ;;[0.15 0.15 0.15 0.5] une seule note
    (if (== _returnvalue_2 1)
      (Game|SpawnActorfromClass "/Game/Blueprint/RythmGame/BP_MusicNote.BP_MusicNote_C" (Transformation|GetWorldTransform (Variables|Default|GetArrow%201)) "Undefined" "MultiplyWithRoot" 0 0)
      (elif (== _returnvalue_2 2)
        (Game|SpawnActorfromClass "/Game/Blueprint/RythmGame/BP_MusicNote.BP_MusicNote_C" (Transformation|GetWorldTransform (Variables|Default|GetArrow%202)) "Undefined" "MultiplyWithRoot" 0 0)
        (else
          (Game|SpawnActorfromClass "/Game/Blueprint/RythmGame/BP_MusicNote.BP_MusicNote_C" (Transformation|GetWorldTransform (Variables|Default|GetArrow%203)) "Undefined" "MultiplyWithRoot" 0 0))))
    (else
      ;;[0.15 0.15 0.15 0.5] 2 notes
      (if (== _returnvalue 1)
        (Game|SpawnActorfromClass "/Game/Blueprint/RythmGame/BP_MusicNote.BP_MusicNote_C" (Transformation|GetWorldTransform (Variables|Default|GetArrow%201)) "Undefined" "MultiplyWithRoot" 0 0)
        (Game|SpawnActorfromClass "/Game/Blueprint/RythmGame/BP_MusicNote.BP_MusicNote_C" (Transformation|GetWorldTransform (Variables|Default|GetArrow%202)) "Undefined" "MultiplyWithRoot" 0 0)
        (elif (== _returnvalue 2)
          (Game|SpawnActorfromClass "/Game/Blueprint/RythmGame/BP_MusicNote.BP_MusicNote_C" (Transformation|GetWorldTransform (Variables|Default|GetArrow%201)) "Undefined" "MultiplyWithRoot" 0 0)
          (Game|SpawnActorfromClass "/Game/Blueprint/RythmGame/BP_MusicNote.BP_MusicNote_C" (Transformation|GetWorldTransform (Variables|Default|GetArrow%203)) "Undefined" "MultiplyWithRoot" 0 0)
          (else
            (Game|SpawnActorfromClass "/Game/Blueprint/RythmGame/BP_MusicNote.BP_MusicNote_C" (Transformation|GetWorldTransform (Variables|Default|GetArrow%202)) "Undefined" "MultiplyWithRoot" 0 0)
            (Game|SpawnActorfromClass "/Game/Blueprint/RythmGame/BP_MusicNote.BP_MusicNote_C" (Transformation|GetWorldTransform (Variables|Default|GetArrow%203)) "Undefined" "MultiplyWithRoot" 0 0)))))))

(event EventLaunchGame
  ;[0.15 0.15 0.15 0.5] spawn des notes
  (Utilities|Time|SetTimerbyEvent (delegate Custom|music%20note%20spawn) 1.0 true))

(event EventBeginPlay
  ;[0.15 0.15 0.15 0.5] Cast au player
  (bind _asbp_first_person_character (Utilities|Casting|CastToBP_FirstPersonCharacter (Game|GetPlayerCharacter 0)))
  (Variables|Default|SetAs%20BP%20First%20Person%20Character _asbp_first_person_character)
  (Variables|Default|SetBase%20material (Rendering|Material|GetMaterial (Variables|Default|GetTempoBar) 0)))

(fn ConstructionScript)

(fn FeedbackBPScreen)